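; BP_BikeRider is a player-controlled bike rider character that moves relative to the control rotation's yaw.
; The Pedal axis event calls LaunchCharacter along yaw-only forward by SpeedValue, ignoring axis value, adding to horizontal velocity and overriding vertical velocity.
; The Steer Left Right axis adds sideways movement input along the yaw-only right vector.
; The Left Shift press leads to an empty branch, and the construction script is empty.
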(event Input|AxisEvents|InputAxisSteerLeftRight
  (params (AxisValue :type Float%20%28single-precision%29))
  (Pawn|Input|AddMovementInput (Math|Vector|GetRightVector (Math|Rotator|MakeRotator 0.0 0.0 (.Yaw (Math|Rotator|BreakRotator (Pawn|GetControlRotation :!class /Script/Engine.Pawn))))) AxisValue false))

(event Input|AxisEvents|InputAxisPedal
  (params (AxisValue :type Float%20%28single-precision%29))
  (Character|LaunchCharacter (* (Math|Vector|GetForwardVector (Math|Rotator|MakeRotator 0.0 0.0 (.Yaw (Math|Rotator|BreakRotator (Pawn|GetControlRotation :!class /Script/Engine.Pawn))))) (Variables|Default|GetSpeedValue)) false true))

(event Input|KeyboardEvents|LeftShift
  (params (Key :type Key%20Structure :default "None"))
  (:Pressed
    (if true
      _)))

(fn ConstructionScript)