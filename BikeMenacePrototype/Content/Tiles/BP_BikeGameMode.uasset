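; Bike game mode that builds a straight floor track from randomly chosen tile Blueprints.
; AddFloor spawns one of three tile classes at FloorAttachPoint, then moves that point a fixed distance along world X.
; ExtendFloor adds a tile and destroys the oldest once the FloorTiles array exceeds NumberOfTiles, forming a rolling window.
; BeginPlay calls both functions in a loop to seed the track, then casts the player pawn to Bike without using it.
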(event EventBeginPlay
  (for _index (range 0 (- (Variables|Default|GetNumberOfTiles) 1))
    (CallFunction|AddFloor)
    (CallFunction|ExtendFloor))
  (Utilities|Casting|CastToBike (Game|Player|GetPlayerPawn 0)))

(event EventTick
  (params (DeltaSeconds :type Float%20%28single-precision%29)))

(fn ConstructionScript)

(fn AddFloor
  (bind _returnvalue (Game|SpawnActorfromClass (Utilities|Select :Index (Math|Random|RandomIntegerinRange 0 2) :Option%200 "/Game/Tiles/Tile1.Tile1_C" :Option%201 "/Game/Tiles/Tile2.Tile2_C" :Option%202 "/Game/Tiles/Tile3.Tile3_C") (Variables|Default|GetFloorAttachPoint) "Undefined" 0 0))
  (Variables|Default|SetFloorAttachPoint (Math|Conversions|ToTransform(Vector) (+ (.Location (Math|Transform|BreakTransform (Transformation|GetActorTransform _returnvalue))) "1500.000000, 0, 0")))
  (Utilities|Array|Add (Variables|Default|GetFloorTiles) 0))

(fn ExtendFloor
  (bind _floortiles (Variables|Default|GetFloorTiles))
  (bind _output (Utilities|Array|Get(acopy) _floortiles))
  (CallFunction|AddFloor)
  (if (> (Utilities|Array|Length (Variables|Default|GetFloorTiles)) (+ 0 (Variables|Default|GetNumberOfTiles)))
    (Actor|DestroyActor _output)
    (Utilities|Array|RemoveItem _floortiles _output)))